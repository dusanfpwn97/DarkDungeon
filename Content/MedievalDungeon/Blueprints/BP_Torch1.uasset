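; Torch actor for the medieval dungeon that plays fire audio and tracks the player's presence near it.
; On BeginPlay it waits a random short delay, likely to stagger multiple torches, then plays a looping fire sound at its location.
; Overlap begin and end events increment and decrement LightCount on the FirstPersonCharacter, counting overlapping light sources, and print the new value to screen.
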(event EventBeginPlay
  (Utilities|FlowControl|Delay (Math|Random|RandomFloatinRange 0.0 3.0))
  (Audio|PlaySoundatLocation "/Game/fireNoCrackingLoop.fireNoCrackingLoop" (Transformation|GetActorLocation) "0, 0, 0" 1.0 1.0 0.0 0 0 0))

(event Collision|EventActorBeginOverlap
  (params (OtherActor :type Actor%20Object%20Reference))
  (bind _asfirst_person_character (Utilities|Casting|CastToFirstPersonCharacter OtherActor))
  (bind _output_get (Variables|/Game/FirstPersonBP/Blueprints/FirstPersonCharacter.FirstPersonCharacter_C|SetLightCount _asfirst_person_character (+ (Variables|/Game/FirstPersonBP/Blueprints/FirstPersonCharacter.FirstPersonCharacter_C|GetLightCount _asfirst_person_character) 1)))
  (Development|PrintString (Utilities|String|ToString(Integer) _output_get)))

(event EventTick
  (params (DeltaSeconds :type Float%20%28single-precision%29)))

(event Collision|EventActorEndOverlap
  (params (OtherActor :type Actor%20Object%20Reference))
  (bind _asfirst_person_character (Utilities|Casting|CastToFirstPersonCharacter OtherActor))
  (bind _output_get (Variables|/Game/FirstPersonBP/Blueprints/FirstPersonCharacter.FirstPersonCharacter_C|SetLightCount _asfirst_person_character (+ (Variables|/Game/FirstPersonBP/Blueprints/FirstPersonCharacter.FirstPersonCharacter_C|GetLightCount _asfirst_person_character) -1)))
  (Development|PrintString (Utilities|String|ToString(Integer) _output_get)))

(fn ConstructionScript)
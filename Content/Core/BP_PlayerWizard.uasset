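; Player wizard character with a first/third-person view toggle and a switchable staff light.
; SwitchView changes the camera boom length and hides the mesh in first person.
; ToggleStaffLight flip-flops the point light nested under the StaffLight component and sets AdditionalLightIntensity to match.
; Tick prints the last received light intensity on authority for debugging; ChangeStaffLight is an empty stub.
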(event Custom|ChangeStaffLight)

(event EventBeginPlay)

(event Collision|EventActorBeginOverlap
  (params (OtherActor :type Actor%20Object%20Reference)))

(event EventTick
  (params (DeltaSeconds :type Float%20%28single-precision%29))
  (Networking|SwitchHasAuthority
    (:Authority
      (Development|PrintString (Utilities|String|ToString(Float) (Class|CharBase|GetLastReceivedLightIntensity)) true false "(R=0.000000,G=0.660000,B=1.000000,A=1.000000)" 0.0))))

(event Input|ActionEvents|InputActionSwitchView
  (params (Key :type Key%20Structure :default "None"))
  (bind _cameraboom (Variables|Default|GetCameraBoom))
  (bind _mesh (Variables|Character|GetMesh))
  (bind _cameraboom_2 (Variables|Default|GetCameraBoom))
  (:Pressed
    (bind _output_get (Variables|Default|SetIsInFirstPerson (not (Variables|Default|GetIsInFirstPerson))))
    (if _output_get
      (Variables|/Script/Engine.SpringArmComponent|SetTargetArmLength _cameraboom_2 0.0)
      (Rendering|SetVisibility _mesh false false)
      (Transformation|SetRelativeLocation _cameraboom "0, 0,70.000000" false false)
      (else
        (Variables|/Script/Engine.SpringArmComponent|SetTargetArmLength _cameraboom_2 (Variables|Default|GetThirdPersonTargetArmLength))
        (Rendering|SetVisibility _mesh true false)
        (Transformation|SetRelativeLocation _cameraboom "0, 0,70.000000" false false)))))

(event Input|ActionEvents|InputActionToggleStaffLight
  (params (Key :type Key%20Structure :default "None"))
  (:Pressed
    (Utilities|FlowControl|FlipFlop
      (:A
        (bind _aspoint_light_component (Utilities|Casting|CastToPointLightComponent (Components|GetChildComponent (Components|GetChildComponent (Variables|Default|GetStaffLight) 0) 0)))
        (Rendering|SetVisibility _aspoint_light_component false false)
        (Variables|Default|SetAdditionalLightIntensity 0.0))
      (:B
        (bind _aspoint_light_component_2 (Utilities|Casting|CastToPointLightComponent (Components|GetChildComponent (Components|GetChildComponent (Variables|Default|GetStaffLight) 0) 0)))
        (Rendering|SetVisibility _aspoint_light_component_2 true false)
        (Variables|Default|SetAdditionalLightIntensity 1.0)))))

(fn ConstructionScript)
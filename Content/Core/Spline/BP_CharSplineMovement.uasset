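; Character that walks along an assigned spline path in a continuous loop using AI MoveTo, started on BeginPlay.
; A fast looping timer re-issues the move toward a point on the spline, advancing that point when the character gets near it and wrapping to the start past the end.
; Both the look-ahead step and arrival threshold scale with max movement speed.
; Tick prints the light received from EnviromentStats as on-screen debug.
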(event Custom|MovementLoopTimer
  (CallFunction|MovementLoop))

(event Custom|StopTheMovementLoop
  (Variables|Movement|SetShouldMove false)
  (if (Utilities|Time|IsValidTimerHandle (Variables|Movement|GetMovementLoopHandle))
    (Utilities|Time|ClearandInvalidateTimerbyHandle (Variables|Movement|GetMovementLoopHandle))))

(event Custom|StartTheMovementLoop
  (Variables|Movement|SetShouldMove true)
  (Utilities|IsValid (Variables|Movement|GetMovementPathToFollow)
    (:Is%20Valid
      (Variables|Movement|SetCurrentLocationToMoveTo (Spline|GetLocationatDistanceAlongSpline (Variables|/Game/Core/Spline/BP_SplineMovementPath.BP_SplineMovementPath_C|GetSplinePath (Variables|Movement|GetMovementPathToFollow)) (Variables|Movement|GetTargetDistanceAlongTheMovementPath) "World"))
      (bind _returnvalue (Utilities|Time|SetTimerbyEvent (delegate Custom|MovementLoopTimer) 0.02 true))
      (Variables|Movement|SetMovementLoopHandle _returnvalue))
    (:Is%20Not%20Valid
      (Development|PrintString (Utilities|String|Append (Utilities|GetDisplayName self) " is trying to move, but the movement path is not set!")))))

(event Custom|MovementLoop
  (Variables|Movement|SetCurrentLocationToMoveTo (CallFunction|GetLocationtoMoveto))
  (AI|AIMoveTo self (Variables|Movement|GetCurrentLocationToMoveTo) 0 5.0 false))

(event EventBeginPlay
  (CallFunction|StarttheMovementLoop))

(event EventTick
  (params (DeltaSeconds :type Float%20%28single-precision%29))
  (bind _returnvalue (Class|EnviromentStats|CalculateLightReceived (Variables|Default|GetEnviromentStats) self))
  (Development|PrintString (Utilities|String|ToString(Float) _returnvalue) true false "(R=0.000000,G=0.660000,B=1.000000,A=1.000000)" 0.0))

(fn ConstructionScript)

(fn IsNeartheTargetMovementLocation
  (return (<= (Math|Vector|Distance(Vector) (Variables|Movement|GetCurrentLocationToMoveTo) (Transformation|GetActorLocation)) (* (Class|MovementComponent|GetMaxSpeed (Variables|Character|GetCharacterMovement)) (Variables|MovementSetup|GetFollowPathStifness)))))

(fn SetANewMovementLocation
  (bind _output_get (Variables|Movement|SetTargetDistanceAlongTheMovementPath (+ (Variables|Movement|GetTargetDistanceAlongTheMovementPath) (* (Class|MovementComponent|GetMaxSpeed (Variables|Character|GetCharacterMovement)) (Variables|MovementSetup|GetMovementTargetDistanceMultiplier)))))
  (if (> _output_get (Spline|GetSplineLength (Variables|/Game/Core/Spline/BP_SplineMovementPath.BP_SplineMovementPath_C|GetSplinePath (Variables|Movement|GetMovementPathToFollow))))
    (Variables|Movement|SetTargetDistanceAlongTheMovementPath 0.0))
  (return (Spline|GetLocationatDistanceAlongSpline (Variables|/Game/Core/Spline/BP_SplineMovementPath.BP_SplineMovementPath_C|GetSplinePath (Variables|Movement|GetMovementPathToFollow)) (Variables|Movement|GetTargetDistanceAlongTheMovementPath) "World")))

(fn GetLocationtoMoveto
  (if (CallFunction|IsNeartheTargetMovementLocation)
    (bind _newmovementlocation (CallFunction|SetANewMovementLocation))
    (return _newmovementlocation)
    (else
      (return (Variables|Movement|GetCurrentLocationToMoveTo)))))
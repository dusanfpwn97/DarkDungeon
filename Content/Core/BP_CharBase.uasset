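; Base character Blueprint that currently acts as a test harness for the statistics component and a test UI.
; BeginPlay creates the WBP_Test widget and adds it to the viewport.
; Every Tick, it passes the difference between a time-based absolute sine wave and the current Stealth value to StatisticsComp.ModifyStatistic, making Stealth oscillate between zero and one hundred.
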(event EventBeginPlay
  (bind _returnvalue (UserInterface|CreateWidget "/Game/Core/UI/WBP_Test.WBP_Test_C"))
  (UserInterface|Viewport|AddtoViewport _returnvalue 0))

(event Collision|EventActorBeginOverlap
  (params (OtherActor :type Actor%20Object%20Reference)))

(event EventTick
  (params (DeltaSeconds :type Float%20%28single-precision%29))
  (bind _statisticscomp (Variables|Default|GetStatisticsComp))
  (Class|ARSStatisticsComponent|ModifyStatistic _statisticscomp "(TagName=\"RPG.Statistic.Stealth\")" (- (* (Math|Float|Absolute(Float) (Math|Trig|Sin(Radians) (Utilities|Time|GetTimeSeconds))) 1e+02) (Class|ARSStatisticsComponent|GetCurrentValueforStatitstic _statisticscomp "(TagName=\"RPG.Statistic.Stealth\")"))))

(fn ConstructionScript)